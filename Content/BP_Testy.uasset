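; BP_Testy is a player-controlled test pawn or character with basic camera-relative movement and look controls.
; The Foward/Back axis adds movement along the Camera's world forward vector, while the turn and LookUp axes feed controller yaw and pitch.
; An unconnected chain that would create the BP_PLayerWidget HUD and show the mouse cursor never runs, and BeginPlay, Tick and the construction script are empty.
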(event `self.ReceiveBeginPlay`)

(event `InputAxis|Foward/Back`
  (params (AxisValue :type "Float (single-precision)"))
  (`self.AddMovementInput` (`KismetMathLibrary.Conv_RotatorToVector` (`SceneComponent.K2_GetComponentRotation` (`self.Camera`))) AxisValue))

(event `InputAxis|turn`
  (params (AxisValue :type "Float (single-precision)"))
  (`self.AddControllerYawInput` AxisValue))

(event `InputAxis|LookUp`
  (params (AxisValue :type "Float (single-precision)"))
  (`self.AddControllerPitchInput` AxisValue))

(fn `UserConstructionScript`)